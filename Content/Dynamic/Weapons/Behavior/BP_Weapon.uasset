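; Weapon actor that fires projectiles on behalf of the Pawn it is attached to, with automatic fire while the trigger is held.
; PullTrigger fires once through a DoOnce and starts a looping timer at the RoundsPerSecond rate, which ReleaseTrigger clears.
; Each shot spawns BP_Projectile2, plays a sound and reports noise with the Pawn as instigator.
; BeginPlay hides the spawn point and adds a reticle widget for player-controlled owners.
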(event Custom|PullTrigger
  (params (ProjectileSpawnPoint :type Transform))
  (Utilities|FlowControl|DoOnce false
    (:Completed
      (CallFunction|Fire ProjectileSpawnPoint)
      (Utilities|Time|SetTimerbyFunctionName 0 "Fire" (/ 1.0 (Variables|Default|GetRoundsPerSecond)) true))))

(event Custom|ReleaseTrigger
  (Utilities|Time|ClearTimerbyFunctionName 0 "Fire")
  (Utilities|FlowControl|DoOnce false) ; enters at Reset
)

(event Custom|Fire
  (params (ProjectileSpawnPoint :type Transform))
  (bind _location (Math|Transform|BreakTransform ProjectileSpawnPoint))
  (bind _aspawn (Utilities|Casting|CastToPawn (Actor|GetAttachParentActor))
    (:then
      (Game|SpawnActorfromClass "/Game/Dynamic/Weapons/Behavior/BP_Projectile2.BP_Projectile2_C" ProjectileSpawnPoint "Undefined" 0 _aspawn)
      (Audio|SpawnSoundatLocation "/Game/Static/Player/Audio/FirstPersonTemplateWeaponFire02.FirstPersonTemplateWeaponFire02" _location)
      (Class|AISenseHearing|ReportNoiseEvent _location 1.0 _aspawn 0.0 "None"))
    (:CastFailed
      (Development|PrintString "Error in weapon fire event: cast failed"))))

(event Collision|EventActorBeginOverlap
  (params (OtherActor :type Actor%20Object%20Reference)))

(event EventBeginPlay
  (Utilities|FlowControl|Delay 1e-05)
  (Development|SetHiddeninGame (Variables|Default|GetProjectileSpawnPoint) true false)
  (bind _aspawn (Utilities|Casting|CastToPawn (Actor|GetAttachParentActor)))
  (if (Pawn|IsPlayerControlled _aspawn)
    (bind _asplayer_controller (Utilities|Casting|CastToPlayerController (Pawn|GetController _aspawn)))
    (bind _returnvalue (UserInterface|CreateWidget "/Game/Dynamic/Weapons/Behavior/FPS_Reticle.FPS_Reticle_C" _asplayer_controller))
    (bind _output_get (Variables|Default|SetTargetReticle _returnvalue))
    (UserInterface|Viewport|AddtoViewport _output_get 0)))

(fn ConstructionScript)