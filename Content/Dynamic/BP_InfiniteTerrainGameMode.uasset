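; Game mode for an infinite terrain game that spawns chained terrain tiles and tracks score.
; On BeginPlay it fills a nav mesh bounds volume pool, then spawns the initial tiles.
; SpawnTile creates a BP_Tile_Child1 at the stored transform, passes it the pool and takes its attach point for the next tile.
; NewTileConquered increments the score; a random BP_Tile spawn branch is left disconnected.
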(event EventBeginPlay
  (Class|InfiniteTerrainGameMode|PopulateBoundsVolumePool)
  (for _index (range 0 3)
    (CallFunction|SpawnTile)))

(event EventTick
  (params (DeltaSeconds :type Float%20%28single-precision%29)))

(fn ConstructionScript)

(fn SpawnTile
  (bind _returnvalue (Game|SpawnActorfromClass "/Game/Dynamic/Terrain/BP_Tile_Child1.BP_Tile_Child1_C" (Variables|Default|GetNextTileTransform) "Undefined" 0 0))
  (Class|Tile|SetPool _returnvalue (Variables|Default|GetNavMeshBoundsVolumePool))
  (Variables|Default|SetNextTileTransform (Default|GetAttachPoint _returnvalue)))

(fn NewTileConquered
  (Math|Integer|IncrementInt (Variables|Default|GetScore)))