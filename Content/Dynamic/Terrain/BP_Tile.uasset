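; Infinite-terrain tile that populates itself on BeginPlay with randomly placed AI pawns, props, trees and rocks, and starts with its gate locked.
; Player overlap with LockCollision opens the gate and animates its dynamic material's opacity; leaving relocks it and turns gate and post-process tint red.
; Player overlap with DestroyCollision asks InfiniteTerrainGameMode to spawn a tile, then destroys this one.
; GetAttachPoint exposes a transform, presumably for chaining tiles.
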(event OnComponentBeginOverlap(DestroyCollision)
  (params (OverlappedComponent :type Primitive%20Component%20Object%20Reference) (OtherActor :type Actor%20Object%20Reference) (OtherComp :type Primitive%20Component%20Object%20Reference) (OtherBodyIndex :type Integer) (bFromSweep :type Boolean) (SweepResult :type Hit%20Result%20Structure%20%28by%20ref%29))
  (Utilities|IsPlayer? OtherActor
    (:True
      (bind _asinfinite_terrain_game_mode (Utilities|Casting|CastToInfiniteTerrainGameMode (Game|GetGameMode)))
      (Default|SpawnTile _asinfinite_terrain_game_mode)
      (Actor|DestroyActor))))

(event OnComponentEndOverlap(LockCollision)
  (params (OverlappedComponent :type Primitive%20Component%20Object%20Reference) (OtherActor :type Actor%20Object%20Reference) (OtherComp :type Primitive%20Component%20Object%20Reference) (OtherBodyIndex :type Integer))
  (Utilities|IsPlayer? OtherActor
    (:True
      (CallFunction|Lock)
      (Utilities|FlowControl|Sequence
        (:then_0
          ;[1 1 1] Pulse Green
          (bind _newtrack_0 (Timeline|Timeline_Opacity Stop)
            (:Update
              (Rendering|Material|SetScalarParameterValue (Variables|Default|GetGateMaterial) "Opacity" _newtrack_0 :!class /Script/Engine.MaterialInstanceDynamic))
            (:Finished
              (Development|PrintString "Hello"))))
        (:then_1
          (CallFunction|SetDoorRed))))))

(event OnComponentBeginOverlap(LockCollision)
  (params (OverlappedComponent :type Primitive%20Component%20Object%20Reference) (OtherActor :type Actor%20Object%20Reference) (OtherComp :type Primitive%20Component%20Object%20Reference) (OtherBodyIndex :type Integer) (bFromSweep :type Boolean) (SweepResult :type Hit%20Result%20Structure%20%28by%20ref%29))
  (Utilities|IsPlayer? OtherActor
    (:True
      (CallFunction|Unlock)
      ;[1 1 1] Pulse Green
      (bind _newtrack_0 (Timeline|Timeline_Opacity Play)
        (:Update
          (Rendering|Material|SetScalarParameterValue (Variables|Default|GetGateMaterial) "Opacity" _newtrack_0 :!class /Script/Engine.MaterialInstanceDynamic))
        (:Finished
          (Development|PrintString "Hello"))))))

(event Collision|EventActorBeginOverlap
  (params (OtherActor :type Actor%20Object%20Reference)))

(event EventBeginPlay
  (CallFunction|Lock)
  (Class|Tile|PlaceAIPawns "/Game/Dynamic/Character/BP_CharacterInC++.BP_CharacterInC++_C" 2 5 1e+02)
  (Class|Tile|PlaceActors "/Game/Dynamic/Terrain/Props/BP_ShippingContainer.BP_ShippingContainer_C" 0 2 5e+02 1.0 1.0)
  (Class|Tile|PlaceActors "/Game/Dynamic/Terrain/Props/BP_Box.BP_Box_C" 0 4 1e+02 1.0 1.0)
  (Class|Tile|PlaceActors "/Game/Dynamic/Terrain/Props/BP_Canister.BP_Canister_C" 0 6 5e+01 1.0 1.0)
  (Class|Tile|PlaceActors "/Game/Dynamic/Terrain/Props/BP_SandbagWall.BP_SandbagWall_C" 0 2 2.5e+02 1.0 1.0)
  (Class|Tile|PlaceActors "/Game/Dynamic/Terrain/Props/BP_TreeAspen.BP_TreeAspen_C" 1 10 1e+02 1.0 1.0)
  (Class|Tile|PlaceActors "/Game/Dynamic/Terrain/Props/BP_Rock1.BP_Rock1_C" 1 3 1.5e+02 1.0 5.0)
  (Class|Tile|PlaceActors "/Game/Dynamic/Terrain/Props/BP_Rock2.BP_Rock2_C" 0 3 2.5e+02 1.0 5.0)
  (Class|Tile|PlaceActors "/Game/Dynamic/Terrain/Props/BP_Rock3.BP_Rock3_C" 0 3 2.5e+02 1.0 5.0))

(fn ConstructionScript
  (bind _returnvalue (Rendering|Material|CreateDynamicMaterialInstance (Variables|Default|GetGate) 0 "/Game/Dynamic/Terrain/MI_Gate.MI_Gate" :!class /Script/Engine.PrimitiveComponent))
  (Variables|Default|SetGateMaterial _returnvalue))

(fn GetAttachPoint
  (return (Transformation|GetWorldTransform (Variables|Default|GetAttachPoint))))

(fn Unlock
  (Collision|SetCollisionEnabled (Variables|Default|GetGate) "NoCollision"))

(fn Lock
  (Collision|SetCollisionEnabled (Variables|Default|GetGate) "QueryAndPhysics"))

(fn GreenGatePulse)

(fn SetDoorRed
  (bind _postprocess (Variables|Default|GetPostProcess))
  (bind _gatematerial (Variables|Default|GetGateMaterial))
  ;[1 1 1] Set door to red
  (Rendering|Material|SetVectorParameterValue _gatematerial "Color" (Math|Color|MakeColor 1.0 0.0 0.0) :!class /Script/Engine.MaterialInstanceDynamic)
  (Rendering|Material|SetScalarParameterValue _gatematerial "Opacity" 1.0 :!class /Script/Engine.MaterialInstanceDynamic)
  (Variables|/Script/Engine.PostProcessComponent|SetSettings _postprocess (Utilities|Struct|MakePostProcessSettings "(R=0.505208,G=0.000000,B=0.000000,A=1.000000)" (.BloomIntensity (Utilities|Struct|BreakPostProcessSettings (Variables|/Script/Engine.PostProcessComponent|GetSettings _postprocess))))))