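; Terrain tile child Blueprint that dresses itself with aspen trees and rocks when play begins.
; After the parent BeginPlay runs, it destroys any attached shipping container actors.
; It then calls PlaceActors for aspens and three rock types, each with its own count and radius settings, with larger maximum scales for rocks.
; An unconnected loop that would add instances at random points within the Floor bounds never runs.
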(event EventBeginPlay
  (|CallParentFunction)
  (for _array_element (Actor|GetAttachedActors)
    (if (Utilities|ClassIsChildOf (Utilities|GetClass _array_element) "/Game/Dynamic/Terrain/Props/BP_ShippingContainer.BP_ShippingContainer_C")
      (Actor|DestroyActor _array_element)))
  (Class|Tile|PlaceActors "/Game/Dynamic/Terrain/Props/BP_TreeAspen.BP_TreeAspen_C" 1 20 8e+01 1.0 1.0)
  (Class|Tile|PlaceActors "/Game/Dynamic/Terrain/Props/BP_Rock1.BP_Rock1_C" 1 3 1.5e+02 1.0 5.0)
  (Class|Tile|PlaceActors "/Game/Dynamic/Terrain/Props/BP_Rock2.BP_Rock2_C" 0 3 2.5e+02 1.0 5.0)
  (Class|Tile|PlaceActors "/Game/Dynamic/Terrain/Props/BP_Rock3.BP_Rock3_C" 0 3 2.5e+02 1.0 5.0))

(event Collision|EventActorBeginOverlap
  (params (OtherActor :type Actor%20Object%20Reference))
  (|CallParentFunction OtherActor) ; This node is disabled and will not be called.\nDrag off pins to build functionality.
)

(event EventTick
  (params (DeltaSeconds :type Float%20%28single-precision%29)))

(fn ConstructionScript
  (|CallParentFunction))